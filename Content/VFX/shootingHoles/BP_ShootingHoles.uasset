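; Shooting-hole VFX actor that places a decal at a random local offset with two accompanying Niagara effects.
; Tick calls MakeHole once the short BeginPlay delay has elapsed and both the Start and DoOnce flags are true, then clears DoOnce.
; MakeHole randomizes X and Z, adds the rotated, scaled decal there, moves both Niagara components to match and activates them.
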(event `self.ReceiveBeginPlay`
  (`KismetSystemLibrary.Delay` 0.2)
  (set `self.Delay` true))

(event `self.ReceiveTick`
  (params (DeltaSeconds :type "Float (single-precision)"))
  (if (`self.Delay`)
    (if (`self.Start`)
      (if (`self.DoOnce`)
        (set `self.DoOnce` false)
        (`self.MakeHole`)))))

(fn `MakeHole`
  (set `self.RandX` (`KismetMathLibrary.RandomFloatInRange` -20.0 20.0))
  (set `self.RandZ` (`KismetMathLibrary.RandomFloatInRange` -20.0 20.0))
  (`AddComponent|NODE_AddDecalComponent-0` :`RelativeTransform` (`KismetMathLibrary.MakeTransform` (`KismetMathLibrary.MakeVector` (`self.RandX`) 0.0 (`self.RandZ`)) (struct :`Yaw` 90.0 :`Roll` 90.0) (0.5 0.02 0.02)))
  (`SceneComponent.K2_SetRelativeLocation` (`self.Niagara`) (`KismetMathLibrary.MakeVector` (`self.RandX`) 0.0 (`self.RandZ`)) false false)
  (`SceneComponent.K2_SetRelativeLocation` (`self.Niagara1`) (`KismetMathLibrary.MakeVector` (`self.RandX`) 0.0 (`self.RandZ`)) false false)
  (`ActorComponent.Activate` (`self.Niagara1`) false)
  (`ActorComponent.Activate` (`self.Niagara`) false))

(fn `UserConstructionScript`)