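; BP_Lights is a traffic-light style prop that shows its state by swapping the emissive material on its light mesh.
; The Color function picks one of three material instances from two booleans: OnLight selects lit or off, and Green selects between the two lit variants.
; Color runs from the construction script and every Tick, with each material swap behind its own DoOnce that has no reset wired.
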(event `self.ReceiveTick`
  (params (DeltaSeconds :type "Float (single-precision)"))
  (`self.Color`))

(fn `Color`
  (bind _fix_light_light_svet_3_1_7c7806a2 (`self.fix_light_Light_svet_3_1_7C7806A2`))
  (if (`self.OnLight`)
    (if (`self.Green`)
      (`/Engine/EditorBlueprintResources/StandardMacros.DoOnce` false
        (:`Completed`
          (`PrimitiveComponent.SetMaterial` _fix_light_light_svet_3_1_7c7806a2 0 "/Game/CustomProps/FixLight/TrafficLightEmissiveMat_Inst3.TrafficLightEmissiveMat_Inst3")))
      (else
        (`/Engine/EditorBlueprintResources/StandardMacros.DoOnce` false
          (:`Completed`
            (`PrimitiveComponent.SetMaterial` _fix_light_light_svet_3_1_7c7806a2 0 "/Game/CustomProps/FixLight/TrafficLightEmissiveMat_Inst1.TrafficLightEmissiveMat_Inst1")))))
    (else
      (`/Engine/EditorBlueprintResources/StandardMacros.DoOnce` false
        (:`Completed`
          (`PrimitiveComponent.SetMaterial` _fix_light_light_svet_3_1_7c7806a2 0 "/Game/CustomProps/FixLight/TrafficLightEmissiveMat_Inst2.TrafficLightEmissiveMat_Inst2"))))))

(fn `UserConstructionScript`
  (`self.Color`))