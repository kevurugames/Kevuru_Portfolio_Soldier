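; Soldier Blueprint that shows or hides the character's head and pistol by swapping mesh material slots to a hidden material.
; HeadVisability swaps the eye, head and helmet slots, using a check bool so materials change only when IsHeadVisible flips.
; PistolVisability swaps one equipment slot from PistolVisible through DoOnce nodes.
; Both run in the construction script and on Tick, where a short Delay precedes the pistol update.
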(event `self.ReceiveTick`
  (params (DeltaSeconds :type "Float (single-precision)"))
  (`self.HeadVisability`)
  (`KismetSystemLibrary.Delay` 0.2)
  (`self.PistolVisability`))

(fn `HeadVisability`
  (bind _soldier_t_pose_v5_2 (`self.Soldier_T-pose_v5_2`))
  (bind _isheadvisible_check (`self.IsHeadVisible_Check`))
  (if (`self.IsHeadVisible`)
    ;[1 1 1] DoOnce
    (if _isheadvisible_check
      (set `self.IsHeadVisible_Check` false)
      (`PrimitiveComponent.SetMaterial` _soldier_t_pose_v5_2 5 "/Game/Soldier/Materials/MI_eyes.MI_eyes")
      (`PrimitiveComponent.SetMaterial` _soldier_t_pose_v5_2 8 "/Game/Soldier/Materials/MI_Head.MI_Head")
      (`PrimitiveComponent.SetMaterial` _soldier_t_pose_v5_2 11 "/Game/Soldier/Materials/MI_Helmet.MI_Helmet")
      (`PrimitiveComponent.SetMaterial` _soldier_t_pose_v5_2 4 "/Game/Soldier/Materials/MI_Eyes_glass.MI_Eyes_glass"))
    (elif (not _isheadvisible_check)
      (set `self.IsHeadVisible_Check` true)
      (`PrimitiveComponent.SetMaterial` _soldier_t_pose_v5_2 5 "/Game/Soldier/Materials/M_Hidden.M_Hidden")
      (`PrimitiveComponent.SetMaterial` _soldier_t_pose_v5_2 8 "/Game/Soldier/Materials/M_Hidden.M_Hidden")
      (`PrimitiveComponent.SetMaterial` _soldier_t_pose_v5_2 11 "/Game/Soldier/Materials/M_Hidden.M_Hidden")
      (`PrimitiveComponent.SetMaterial` _soldier_t_pose_v5_2 4 "/Game/Soldier/Materials/M_Hidden.M_Hidden"))))

(fn `PistolVisability`
  (bind _soldier_t_pose_v5_2 (`self.Soldier_T-pose_v5_2`))
  (if (`self.PistolVisible`)
    (`/Engine/EditorBlueprintResources/StandardMacros.DoOnce` false
      (:`Completed`
        (`PrimitiveComponent.SetMaterial` _soldier_t_pose_v5_2 7 "/Game/Soldier/Materials/MI_eqiup_fastex_knife.MI_eqiup_fastex_knife")))
    (else
      (`/Engine/EditorBlueprintResources/StandardMacros.DoOnce` false
        (:`Completed`
          (`PrimitiveComponent.SetMaterial` _soldier_t_pose_v5_2 7 "/Game/Soldier/Materials/M_Hidden.M_Hidden"))))))

(fn `UserConstructionScript`
  (`self.HeadVisability`)
  (`self.PistolVisability`))