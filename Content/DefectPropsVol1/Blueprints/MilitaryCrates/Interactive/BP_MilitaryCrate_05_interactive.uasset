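; Interactive military crate prop whose lid the player opens and closes with F while inside its box trigger.
; Entering the trigger adds a "Press F" text render prompt; leaving blanks it and starts a delayed auto-close that retries while the lid is moving.
; Open and close timelines drive the lid's roll, with a Finished flag blocking input mid-animation.
; The construction script sizes the trigger and applies color and roughness material parameters.
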(event `self.Box.OnComponentBeginOverlap`
  (params (OverlappedComponent :type "PrimitiveComponent Object Reference") (OtherActor :type "Actor Object Reference") (OtherComp :type "PrimitiveComponent Object Reference") (OtherBodyIndex :type Integer) (bFromSweep :type Boolean) (SweepResult :type "HitResult Structure (by ref)"))
  (set `self.Inbox` true)
  ;[1 1 1] Text_Print
  (bind _returnvalue (`AddComponent|NODE_AddTextRenderComponent-3`))
  (`TextRenderComponent.K2_SetText` _returnvalue "Press \"F\"")
  (`TextRenderComponent.SetHorizontalAlignment` _returnvalue "EHTA_Center")
  (`TextRenderComponent.SetVerticalAlignment` _returnvalue "EVRTA_TextTop"))

(event `self.Box.OnComponentEndOverlap`
  (params (OverlappedComponent :type "PrimitiveComponent Object Reference") (OtherActor :type "Actor Object Reference") (OtherComp :type "PrimitiveComponent Object Reference") (OtherBodyIndex :type Integer))
  (set `self.Inbox` false)
  (`|ExecutionSequence`
    (:`then_0`
      ;[1 1 1] Text_Print
      (`TextRenderComponent.K2_SetText` (stale `self.Box.OnComponentBeginOverlap` _returnvalue) ""))
    (:`then_1`
      ;[1 1 1] Close_Timer
      (`KismetSystemLibrary.Delay` (`KismetMathLibrary.Abs` (`self.Delay`)) :!label _label)
      (if (`self.Finished`)
        (if (`self.Open`)
          (set `self.Finished` false)
          (set `self.Open` false :!label _label_2)
          (bind (_direction _newtrack_0) (`Timeline|Close_Anim` :!via `PlayFromStart`)
            (:`Update`
              (`SceneComponent.K2_SetRelativeRotation` (`self.SM_MilitaryCrateTop_05`) (`KismetMathLibrary.MakeRotator` (* _newtrack_0 -1.0)) false false))
            (:`Finished`
              (set `self.Finished` true))))
        (else
          (goto _label))))))

(event `Key|F` :consume false
  (params (Key :type "Key Structure"))
  (:`Pressed`
    (if (`self.Inbox`)
      (if (`self.Finished`)
        (set `self.Finished` false)
        (if (`self.Open`)
          (goto _label_2)
          (else
            (set `self.Open` true)
            (bind (_direction _newtrack_0) (`Timeline|Open_Anim` :!via `PlayFromStart`)
              (:`Update`
                (`SceneComponent.K2_SetRelativeRotation` (`self.SM_MilitaryCrateTop_05`) (`KismetMathLibrary.MakeRotator` (* _newtrack_0 -1.0)) false false))
              (:`Finished`
                (set `self.Finished` true)))))))))

(fn `UserConstructionScript`
  (bind _box (`self.Box`))
  (bind _sm_militarycratetop_05 (`self.SM_MilitaryCrateTop_05`))
  (`BoxComponent.SetBoxExtent` _box (`KismetMathLibrary.Conv_DoubleToVector` (`self.TrigerSize`)) true)
  (`SceneComponent.K2_SetRelativeTransform` _box (`KismetMathLibrary.Conv_VectorToTransform` (`KismetMathLibrary.MakeVector` 0.0 0.0 (`self.TrigerSize`))) false false)
  (`MeshComponent.SetVectorParameterValueOnMaterials` _sm_militarycratetop_05 "Colorize" (`KismetMathLibrary.Conv_LinearColorToVector` (`self.color`)))
  (`MeshComponent.SetVectorParameterValueOnMaterials` (`self.SM_MilitaryCrate_05`) "Colorize" (`KismetMathLibrary.Conv_LinearColorToVector` (`self.color`)))
  (`MeshComponent.SetScalarParameterValueOnMaterials` _sm_militarycratetop_05 "RoughnessMin" (`self.RoughnessMin`))
  (`MeshComponent.SetScalarParameterValueOnMaterials` (`self.SM_MilitaryCrate_05`) "RoughnessMin" (`self.RoughnessMin`))
  (`MeshComponent.SetScalarParameterValueOnMaterials` _sm_militarycratetop_05 "RoughnessMax" (`self.RoughnessMax`))
  (`MeshComponent.SetScalarParameterValueOnMaterials` (`self.SM_MilitaryCrate_05`) "RoughnessMax" (`self.RoughnessMax`)))