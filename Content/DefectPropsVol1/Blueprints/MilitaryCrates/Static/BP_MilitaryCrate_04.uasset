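; BP_MilitaryCrate_04 is a configurable military crate prop built from a base mesh and a separate top mesh.
; Its Construction Script rotates the top from the Open (roll) and Rotation (yaw) variables to pose the lid.
; It also pushes a color tint and roughness min/max to both meshes' material parameters.
; The event graph holds only disabled placeholder events, so the prop has no runtime logic.
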(fn `UserConstructionScript`
  (bind _sm_militarycrate_04 (`self.SM_MilitaryCrate_04`))
  (`SceneComponent.K2_SetRelativeRotation` (`self.SM_MilitaryCrateTop_04`) (`KismetMathLibrary.MakeRotator` (* (`self.open`) -180.0) 0.0 (* (`self.rotation`) 60.0)) false false)
  (`MeshComponent.SetVectorParameterValueOnMaterials` _sm_militarycrate_04 "Colorize" (`KismetMathLibrary.Conv_LinearColorToVector` (`self.Color`)))
  (`MeshComponent.SetVectorParameterValueOnMaterials` (`self.SM_MilitaryCrateTop_04`) "Colorize" (`KismetMathLibrary.Conv_LinearColorToVector` (`self.Color`)))
  (`MeshComponent.SetScalarParameterValueOnMaterials` _sm_militarycrate_04 "RoughnessMin" (`self.RoughnessMin`))
  (`MeshComponent.SetScalarParameterValueOnMaterials` (`self.SM_MilitaryCrateTop_04`) "RoughnessMin" (`self.RoughnessMin`))
  (`MeshComponent.SetScalarParameterValueOnMaterials` _sm_militarycrate_04 "RoughnessMax" (`self.RoughnessMax`))
  (`MeshComponent.SetScalarParameterValueOnMaterials` (`self.SM_MilitaryCrateTop_04`) "RoughnessMax" (`self.RoughnessMax`)))